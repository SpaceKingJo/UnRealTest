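; HeroBP is a hero Blueprint that places a marker actor wherever the player left-clicks in the world.
; On BeginPlay it spawns a MousePointBP at its own location, stores it as MouseClickPoint and shows the mouse cursor.
; Each left-click traces under the cursor on the Visibility channel and moves that marker to the hit location, without checking for a hit.
; The graph contains no logic that moves the hero itself.
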(event EventBeginPlay
  (bind _returnvalue (Game|SpawnActorfromClass "/Game/UI/MousePointBP.MousePointBP_C" (Math|Conversions|ToTransform(Vector) (Transformation|GetActorLocation)) "Undefined" 0 0))
  (Variables|컴포넌트|SetMouseClickPoint _returnvalue)
  (Variables|/Script/Engine.PlayerController|SetbShowMouseCursor (Game|GetPlayerController 0) true))

(event Collision|EventActorBeginOverlap
  (params (OtherActor :type Actor%20Object%20Reference)))

(event EventTick
  (params (DeltaSeconds :type Float%20%28single-precision%29)))

(event Input|ActionEvents|InputActionLeftMouseClicked
  (params (Key :type Key%20Structure :default "AnyKey"))
  (:Pressed
    (Transformation|SetActorLocation (Variables|컴포넌트|GetMouseClickPoint) (.Location (Collision|BreakHitResult (.HitResult (Game|Player|GetHitResultUnderCursorbyChannel (Game|GetPlayerController 0) "TraceTypeQuery1" true)))) false false)))

(fn ConstructionScript)